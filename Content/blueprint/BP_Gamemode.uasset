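; Game mode Blueprint that runs a vanishing-floor minigame where the player wins by outlasting the platform removals.
; StartGame saves platform positions, places the character, then loops through a Delay, recoloring a random platform as warning before teleporting it away.
; Exceeding the removal count triggers Win; Lose has no caller here.
; Both send the character back, stop the loop and restore platforms, Win after a pause.
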(event `StartGame`
  (bind _character (`self.Character`))
  (bind _output (`|GetArrayItem` (`self.platform`) (`self.FloorNum`)))
  (`self.reset`)
  (for (_ _array_index) (`self.platform`)
    (`KismetArrayLibrary.Array_Set` (`self.TranasformArray`) _array_index (`self.K2_GetActorLocation` (`|GetArrayItem` (`self.platform`) _array_index))))
  (`self.K2_SetActorLocation` _character (-100.0 -100.0 910.0) false false)
  (`self.K2_SetActorRotation` :`self` _character)
  (if (<= (`self.counter`) 25) :!label _label
    (if (`self.FlagGameRunning`)
      (set `self.FloorNum` (`KismetMathLibrary.RandomIntegerInRange` 0 35))
      (`PrimitiveComponent.SetMaterial` (`/Game/blueprint/BP_Cube.Cube` _output) 0 "/Game/Models/Material/colorChange.colorChange")
      (`KismetSystemLibrary.Delay` 0.75)
      (`self.K2_TeleportTo` :`self` _output :`DestLocation` (-10000.0 -10000.0 -10000.0))
      (`/Engine/EditorBlueprintResources/StandardMacros.IncrementInt` (`self.counter`)
        (:`  `
          (goto _label))))
    (else
      (`self.Win`))))

(event `reset`
  (set `self.counter` 0)
  (set `self.FlagGameRunning` true)
  (set `self.FloorNum` 0))

(event `CleanUp`
  (for (_array_element _array_index) (`self.TranasformArray`)
    (bind _output (`|GetArrayItem` (`self.platform`) _array_index))
    (`self.K2_TeleportTo` :`self` _output :`DestLocation` _array_element)
    (`PrimitiveComponent.SetMaterial` (`/Game/blueprint/BP_Cube.Cube` _output) 0 "/Game/Models/Material/defaultColor.defaultColor")))

(event `Win`
  (bind _character (`self.Character`))
  (`KismetSystemLibrary.PrintString` "Congratulation!! You Won!!" true false (struct :`G` 0.66 :`B` 1.0 :`A` 1.0) 10.0)
  (`KismetSystemLibrary.Delay` 5.0)
  (`self.K2_TeleportTo` :`self` _character :`DestLocation` (-5870.0 -380.0 878.0) :!label _label_2)
  (`self.K2_SetActorRotation` :`self` _character)
  (set `self.FlagGameRunning` false)
  (`self.CleanUp`))

(event `Lose`
  (`KismetSystemLibrary.PrintString` "You Lost. Better luck next time." true true (struct :`G` 0.66 :`B` 1.0 :`A` 1.0) 10.0)
  (goto _label_2))

(fn `UserConstructionScript`)